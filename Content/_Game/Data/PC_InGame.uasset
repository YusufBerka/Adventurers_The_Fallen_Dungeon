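; In-game player controller that takes each player from lobby character selection into play.
; On begin play, a client RPC adds the input mapping, creates the HUD and lobby widgets, and shows the lobby in UI-only mode.
; Selection goes through a server RPC to GM_InGame, with helpers to spawn and possess the pawn and swap lobby for HUD.
; HP updates retry until the HUD exists, and F10 quits.
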(event `self.ReceiveBeginPlay`
  ;[0 0 0] Initialize Input and UI
  (`self.Client_InitializeInputAndUI`))

(event `Client_InitializeInputAndUI`
  ;[0 0 0] Initialize Input and UI
  (`EnhancedInputSubsystemInterface.AddMappingContext` (subsystem `EnhancedInputLocalPlayerSubsystem`) "/Game/_Game/Inputs/IMC.IMC" 0 (struct)) ; Only running on client
  (bind _returnvalue (`|CreateWidget` "/Game/_Game/Blueprints/UI/UI_Layout.UI_Layout_C" null self))
  (set `self.UI_Layout` _returnvalue)
  (bind _returnvalue_2 (`|CreateWidget` "/Game/_Game/Blueprints/UI/UI_LobbyRoom.UI_LobbyRoom_C"))
  (bind _output_get (set `self.UI_LobbyRoom` _returnvalue_2))
  (`UserWidget.AddToViewport` _output_get 0)
  (`WidgetBlueprintLibrary.SetInputMode_UIOnlyEx` self (`self.UI_LobbyRoom`))
  (set `self.bShowMouseCursor` true))

(event `Client_UpdateHP`
  (params (CurHP :type "Float (double-precision)") (MaxHP :type "Float (double-precision)"))
  ;[0 0 0] Client - Update HP
  (bind _ui_layout (`self.UI_Layout` :!label _label)
    (:`then`
      (`/Game/_Game/Blueprints/UI/UI_Layout.UpdateHP` _ui_layout CurHP MaxHP))
    (:`else`
      (`KismetSystemLibrary.Delay` 0.2)
      (goto _label))))

(event `Server_SelectCharacter`
  (params (PlayerCharacter :type "/Game/_Game/Blueprints/Players/BP_PlayerBase Class Reference"))
  ;[0 0 0] Spawn request from game mode based on info from UI_LobbyRoom
  (bind _asgm_in_game (cast `/Game/_Game/Data/GM_InGame` (`GameplayStatics.GetGameMode`)))
  (`/Game/_Game/Data/GM_InGame.GM_RequestSpawningPlayerCharacter` _asgm_in_game self PlayerCharacter))

(event `Key|F10`
  (params (Key :type "Key Structure"))
  ;[1 0 0] Quit
  (:`Pressed`
    (`KismetSystemLibrary.QuitGame` self "Quit")))

(fn `SpawnCharacterByGameMode`
  (params (Class :type "/Game/_Game/Blueprints/Players/BP_PlayerBase Class Reference") (`Spawn Transform Location` :type "Vector Structure"))
  (bind _returnvalue (`|SpawnActorFromClass` Class (`KismetMathLibrary.MakeTransform` `Spawn Transform Location`) "AdjustIfPossibleButAlwaysSpawn" "MultiplyWithRoot" null null))
  (`self.Possess` _returnvalue))

(fn `TransitionFromSelectionToGame`
  (bind _ui_layout (`self.UI_Layout`))
  (set `self.bShowMouseCursor` false) ; Hide cursor
  (`/Game/_Game/Blueprints/UI/UI_Layout.StartFadingOut` _ui_layout)
  (`UserWidget.AddToViewport` _ui_layout 0) ; Display UI layout
  (`Widget.RemoveFromParent` (`self.UI_LobbyRoom`)) ; Delete selection ui
  (`WidgetBlueprintLibrary.SetInputMode_GameOnly` self) ; Set focus on viewport, don't need to click at the beginning
)

(fn `UserConstructionScript`)