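; Base character Blueprint that provides shared networked damage text, sound broadcast and sprite facing.
; A server event spawns a damage text actor above the given target and multicasts the number, colored by whether this character has the enemy tag.
; Sounds route through a server event to a multicast that plays them at a location on all clients.
; A RepNotify on orientation rotates the sprite to face left or right.
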(event `Server_SpawnDmgTextActor`
  (params (Instigator :type "Actor Object Reference") (DamageNumber :type "Float (double-precision)"))
  (bind _output_get (set `self.DamagedTarget` Instigator))
  (bind (_returnvalue_x _returnvalue_y _returnvalue_z) (`KismetMathLibrary.BreakVector` (`self.K2_GetActorLocation` _output_get)))
  (bind _returnvalue (`|SpawnActorFromClass` "/Game/_Game/Blueprints/BPA/BPA_DamageText.BPA_DamageText_C" (`KismetMathLibrary.MakeTransform` (`KismetMathLibrary.MakeVector` _returnvalue_x _returnvalue_y (+ _returnvalue_z 30.0))) "Undefined" "MultiplyWithRoot" null null)) ; Only server
  (`/Game/_Game/Blueprints/BPA/BPA_DamageText.Multicast_UpdateDmgNumber` _returnvalue DamageNumber (select `bool` (`self.ActorHasTag` "enemy") :`false` (struct :`R` 1.0 :`G` 1.0 :`B` 1.0 :`A` 1.0) :`true` (struct :`R` 1.0 :`G` 0.517657 :`A` 1.0) :!type "LinearColor Structure")))

(event `Server_BroadcastSound`
  (params (Sound :type "SoundBase Object Reference") (Location :type "Vector Structure"))
  ;[0 0 0] Play sound for multiplayer
  (`self.Multicast_BroadcastSound` Sound Location))

(event `Multicast_BroadcastSound`
  (params (Sound :type "SoundBase Object Reference") (Location :type "Vector Structure"))
  ;[0 0 0] Play sound for multiplayer
  (`GameplayStatics.SpawnSoundAtLocation` Sound Location (struct) 1.0 1.0 0.0 null null) ; For single player
)

(fn `OnRep_E_Orientation`
  (bind _sprite (`self.Sprite`))
  (switch `/Game/_Game/Data/Enumerations/E_Orientation` (`self.E_Orientation`)
    (:`NewEnumerator1`
      (`SceneComponent.K2_SetRelativeRotation` :`self` _sprite) ; Right
    )
    (:`NewEnumerator2`
      (`SceneComponent.K2_SetRelativeRotation` _sprite (struct :`Yaw` 180.0) false false) ; Left
    )))

(fn `UserConstructionScript`)