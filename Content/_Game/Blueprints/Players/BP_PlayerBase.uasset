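; Base player character for a multiplayer 2D side-scroller, handling movement, jumping, rolling, attacking, damage, death and revival.
; Input goes through server RPCs and multicasts, with client-side roll prediction and timeline movement stopped by obstacle traces.
; Hits update HP on the player controller and trigger knockback with blinking invincibility, while RepNotifies handle death, respawn location and revive.
; A separately spawned camera follows smoothly, and child classes implement attack collision.
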(event `EnhancedInput|/Game/_Game/Inputs/IA_Movement`
  (params (ActionValue :type "Float (double-precision)") (ElapsedSeconds :type "Float (double-precision)") (TriggeredSeconds :type "Float (double-precision)") (InputAction :type "InputAction Object Reference" :default "/Game/_Game/Inputs/IA_Movement.IA_Movement"))
  ;[0 0 0] Movement & Camera
  (:`Triggered`
    (`self.CanMove`)
    (`self.AddMovementInput` (`KismetMathLibrary.GetForwardVector` (`self.GetControlRotation`)) ActionValue)
    (if (!= ActionValue 0.0)
      (if (> ActionValue 0.0)
        (`self.Server_SetOrientation` "NewEnumerator1")
        (else
          (`self.Server_SetOrientation` "NewEnumerator2"))))))

(event `Server_SetOrientation`
  (params (Orientation :type "/Game/_Game/Data/Enumerations/E_Orientation Enum" :default "NewEnumerator0"))
  ;[0 0 0] Movement & Camera
  (set `self.E_Orientation` Orientation))

(event `UpdateCameraPosition`
  ;[0 0 0] Movement & Camera
  (bind (_direction _alpha) (`Timeline|TL_SmoothingCameraMovement` :!via `PlayFromStart`)
    (:`Update`
      (bind _playercamera (`self.PlayerCamera`)
        (:`then`
          (`self.K2_SetActorLocation` _playercamera (`KismetMathLibrary.VLerp` (`self.K2_GetActorLocation` (`self.PlayerCamera`)) (`self.K2_GetActorLocation`) _alpha) false false))
        (:`else`)))))

(event `EnhancedInput|/Game/_Game/Inputs/IA_Roll`
  (params (ActionValue :type Boolean) (ElapsedSeconds :type "Float (double-precision)") (TriggeredSeconds :type "Float (double-precision)") (InputAction :type "InputAction Object Reference" :default "/Game/_Game/Inputs/IA_Roll.IA_Roll"))
  ;[0 0 0] Rolling Action
  (:`Started`
    (`self.CanRoll`)
    (`self.Server_Rolling`)
    (`/Engine/EditorBlueprintResources/ActorMacros.Switch Has Authority`
      (:`Remote`
        (`PaperZDPlaySlotOverrideAction.PlayAnimationOverrideWithCallbacks` (`PaperZDAnimationComponent.AnimInstance` (`self.AnimationComponent`)) (`self.RollingAnim`) "MyAnimSlot"
          (:`then`
            (`self.TargetedRollingLocation`)))))))

(event `Server_Rolling`
  ;[0 0 0] Rolling Action
  (`self.CanRoll`)
  (set `self.isRolling` true)
  (`self.Multicast_PlayAnimation` (`self.RollingAnim`)) ; Broadcasting animations to all clients
  (`self.CalculateRollingTargetLocation` :!label _label)
  (bind (_direction _alpha) (`Timeline|TL_Rolling` :!via `PlayFromStart`)
    (:`Update`
      (`self.K2_SetActorLocation` (`KismetMathLibrary.VLerp` (`self.K2_GetActorLocation`) (`self.RollingTargetLocation`) _alpha))
      (`self.CheckObstacles`))))

(event `Multicast_PlayAnimation`
  (params (AnimSequence :type "PaperZDAnimSequence Object Reference"))
  ;[0 0 0] Rolling Action
  (`PaperZDPlaySlotOverrideAction.PlayAnimationOverrideWithCallbacks` (`PaperZDAnimationComponent.AnimInstance` (`self.AnimationComponent`)) AnimSequence "MyAnimSlot"))

(event `Server_ResetRolling`
  ;[0 0 0] Rolling Action
  (set `self.isRolling` false) ; Not need to multicast, it's replicated already
)

(event `TargetedRollingLocation`
  ;[0 0 0] Rolling Action
  (goto _label))

(event `ResetRolling`
  ;[0 0 0] Rolling Action
  (set `self.isRolling` false) ; Execute it locally
  (`self.Server_ResetRolling`))

(event `StopIfRolling`
  ;[0 0 0] Rolling Action
  (`TimelineComponent.Stop` (`self.TL_Rolling`)))

(event `EnhancedInput|/Game/_Game/Inputs/IA_Atk`
  (params (ActionValue :type Boolean) (ElapsedSeconds :type "Float (double-precision)") (TriggeredSeconds :type "Float (double-precision)") (InputAction :type "InputAction Object Reference" :default "/Game/_Game/Inputs/IA_Atk.IA_Atk"))
  ;[0 0 0] Attack Action
  (:`Started`
    (`self.CanAtk`)
    (`self.Server_Attack`)))

(event `Server_Attack`
  ;[0 0 0] Attack Action
  (`self.CanAtk`)
  (set `self.isAttacking` true)
  (`|ExecutionSequence`
    (:`then_0`
      (`self.Multicast_PlayAnimation` (`self.AtkAnim`))
      (`KismetSystemLibrary.Delay` 0.8)
      (set `self.AllowMoving` true)
      (set `self.isAttacking` false))
    (:`then_1`
      (`self.AttackCollisionCheck`))))

(event `AttackCollisionCheck`
  ;[0 0 0] Attack Action
)

(event `/Game/_Game/Blueprints/BPI/BPI_Combat.INT_HitHandle`
  (params (Causer :type "Actor Object Reference") (Damage :type "Float (double-precision)") (KnockbackForce :type Integer))
  ;[0 0 0] Hit Handle
  (`/Engine/EditorBlueprintResources/StandardMacros.IsValid` Causer
    (:`Is Valid`
      (set `self.DamageCauser` Causer)
      (set `self.ReceivedDamage` Damage)
      (`self.CanBeDamaged`
        (:`true`
          (`self.Server_SpawnDmgTextActor` self (`self.ReceivedDamage`))
          (bind _alive_ (`self.HandleHitReaction` (`self.ReceivedDamage`)))
          (if _alive_
            (`self.Server_Invincible` (`self.GetKnockBackDirectionAndForce`))
            (else
              (set `self.isDead` true))))))))

(event `Server_Invincible`
  (params (Impulse :type "Vector Structure"))
  ;[0 0 0] Hit Handle
  (`self.Multicast_Invincible` Impulse))

(event `Multicast_Invincible`
  (params (Impulse :type "Vector Structure"))
  ;[0 0 0] Hit Handle
  (set `self.isInvincible` true)
  (bind _returnvalue (`KismetSystemLibrary.K2_SetTimer` null "InvincibleVFX" 0.1 true))
  (set `self.TimerHandle_InvincibleVFX` _returnvalue)
  (`KismetSystemLibrary.K2_SetTimer` null "HandleInvincible" 1.5)
  (`CharacterMovementComponent.AddImpulse` (`self.CharacterMovement`) Impulse true))

(event `Server_InitializationForPlayerStats`
  (`|ExecutionSequence`
    (:`then_0`
      (`KismetSystemLibrary.Delay` 0.05) ; For multiplayer
      (set `self.MaxHP` (`self.PlayerHP`)))
    (:`then_1`
      ;[0 0 0] Get spawn point data from Game Mode
      (bind _asgm_in_game (cast `/Game/_Game/Data/GM_InGame` (`GameplayStatics.GetGameMode`)))
      (set `self.PlayerSpawnLocation` (`/Game/_Game/Data/GM_InGame.InitialSpawnPoint` _asgm_in_game)))))

(event `self.ReceiveBeginPlay`
  (`KismetSystemLibrary.K2_SetTimer` null "CreateCamera" 2.0) ; Give time for client side to initialization
  ;[0 0 0] Preferred way than tick
  (`KismetSystemLibrary.K2_SetTimerDelegate` (`|CreateDelegate` :!event `UpdateCameraPosition`) 0.02 true) ; Bind specific event with timer and call it every 0.02 seconds
  (`self.Server_InitializationForPlayerStats`))

(event `Server_Revive`
  ;[0 0 0] Revive (Run on server
  (set `self.isDead` false))

(event `/Game/_Game/Blueprints/BPI/BPI_Combat.INT_NotMoving`
  (params (AllowMoving :type Boolean))
  ;[0 0 0] Not moving
  (`self.Server_NotMoving` AllowMoving))

(event `Server_NotMoving`
  (params (AllowMoving :type Boolean))
  ;[0 0 0] Not moving
  (`self.Multicast_NotMoving` AllowMoving))

(event `EnhancedInput|/Game/_Game/Inputs/IA_Jump`
  (params (ActionValue :type Boolean) (ElapsedSeconds :type "Float (double-precision)") (TriggeredSeconds :type "Float (double-precision)") (InputAction :type "InputAction Object Reference" :default "/Game/_Game/Inputs/IA_Jump.IA_Jump"))
  ;[0 0 0] Jump Action
  (:`Started`
    (`self.CanDoJump`)
    (`self.Jump`)
    ;;[0 0 0] Legal request
    (`self.Server_BroadcastSound` "/Game/_Game/Assets/Sounds/jump_Cue.jump_Cue" (`self.K2_GetActorLocation`)))
  (:`Canceled`
    (`self.StopJumping` :!label _label_2))
  (:`Completed`
    (goto _label_2)))

(event `Multicast_NotMoving`
  (params (AllowMoving :type Boolean))
  ;[0 0 0] Not moving
  (set `self.AllowMoving` AllowMoving))

(fn `CalculateRollingTargetLocation`
  (set `self.RollingTargetLocation` (+ (`self.K2_GetActorLocation`) (* (`self.GetActorForwardVector`) (select `/Game/_Game/Data/Enumerations/E_Orientation` (`self.E_Orientation`) :`NewEnumerator0` 200 :`NewEnumerator1` 200 :`NewEnumerator2` -200))))
  (return))

(fn `CheckObstacles`
  (bind _returnvalue (`self.K2_GetActorLocation`))
  (bind (_outhit _returnvalue_2) (`KismetSystemLibrary.SphereTraceSingleForObjects` _returnvalue (+ _returnvalue (* (`self.GetActorForwardVector`) (select `/Game/_Game/Data/Enumerations/E_Orientation` (`self.E_Orientation`) :`NewEnumerator0` 50 :`NewEnumerator1` 50 :`NewEnumerator2` -50))) 40.0 (`|MakeArray` "ObjectTypeQuery1" :!type "EObjectTypeQuery Enum")))
  (if _returnvalue_2
    (`TimelineComponent.Stop` (`self.TL_Rolling`))))

(fn `CreateCamera`
  (bind _returnvalue (`|SpawnActorFromClass` "/Game/_Game/Blueprints/BPA/BPA_Camera.BPA_Camera_C" (`KismetMathLibrary.MakeTransform` (`self.K2_GetActorLocation`)) "AdjustIfPossibleButAlwaysSpawn" "MultiplyWithRoot" null null))
  (set `self.PlayerCamera` _returnvalue)
  (bind _aspc_in_game (cast `/Game/_Game/Data/PC_InGame` (`self.GetController`))) ; Possessed by local player controller
  (`PlayerController.SetViewTargetWithBlend` _aspc_in_game (`self.PlayerCamera`) 0.0 "VTBlend_Linear" 0.0 false))

(fn `GetKnockBackDirectionAndForce`
  (returns (ReturnVal :type "Vector Structure"))
  (bind _returnvalue_x (`KismetMathLibrary.BreakVector` (`self.K2_GetActorLocation`)))
  (bind _returnvalue_x_2 (`KismetMathLibrary.BreakVector` (`self.K2_GetActorLocation` (`self.DamageCauser`))))
  (return (`KismetMathLibrary.MakeVector` (select `bool` (<= _returnvalue_x _returnvalue_x_2) :`false` 500.0 :`true` -500.0) 0.0 300.0)))

(fn `HandleHitReaction`
  (params (Dmg :type "Float (double-precision)"))
  (returns (`Alive?` :type Boolean))
  (bind _output_get (set `self.PlayerHP` (`KismetMathLibrary.FClamp` (- (`self.PlayerHP`) Dmg) 0.0 (`self.MaxHP`))))
  (`self.UpdateHPInPlayerBase`) ; After updated hp variables
  (return (> _output_get 0.0)))

(fn `HandleInvincible`
  (set `self.isInvincible` false)
  ;[1 0 0.6023] Same
  (`KismetSystemLibrary.K2_ClearTimer` null "InvincibleVFX")
  ;[0 0 0] Show player character sprite after clear VFX function
  (bind _output_get (set `self.SpriteVisibility` true))
  (`SceneComponent.SetVisibility` (`self.Sprite`) _output_get false))

(fn `INT_CheckAlive`
  (returns (`Alive?` :type Boolean))
  (return (not (`self.isDead`))))

(fn `InvincibleVFX`
  ;[0 0 0] Change its value every 0.1seconds
  (bind _output_get (set `self.SpriteVisibility` (not (`self.SpriteVisibility`))))
  (`SceneComponent.SetVisibility` (`self.Sprite`) _output_get false))

(fn `OnRep_isDead`
  (if (`self.isDead`)
    ;[0 0 0] Play anim
    (`PaperZDAnimInstance.JumpToNode` (`PaperZDAnimationComponent.AnimInstance` (`self.AnimationComponent`)) "death" "Locomotion")
    (else
      ;[1 1 1] Revive
      (set `self.PlayerHP` (`self.MaxHP`)) ; Refill hp
      (`self.UpdateHPInPlayerBase`)
      ;[0 0 0] Remember, they are in Rep/Notify function
      (`self.K2_SetActorLocation` (`self.PlayerSpawnLocation`)) ; Set player character to specific location both on server and client
      (set `self.isInvincible` true)
      (bind _returnvalue (`KismetSystemLibrary.K2_SetTimer` null "InvincibleVFX" 0.1 true))
      (set `self.TimerHandle_InvincibleVFX` _returnvalue)
      (`KismetSystemLibrary.K2_SetTimer` null "HandleInvincible" 1.5))))

(fn `OnRep_MaxHP`
  (`self.UpdateHPInPlayerBase`))

(fn `OnRep_PlayerSpawnLocation`
  (if (not (`self.UpdateRespawnLocation?`))
    (`self.K2_SetActorLocation` (`self.PlayerSpawnLocation`)) ; Set player character to specific location both on server and client
  ))

(fn `UpdateHPInPlayerBase`
  (bind _aspc_in_game (cast `/Game/_Game/Data/PC_InGame` (`self.GetController`)))
  (`/Game/_Game/Data/PC_InGame.Client_UpdateHP` _aspc_in_game (`self.PlayerHP`) (`self.MaxHP`)))

(fn `UserConstructionScript`
  (`parent.UserConstructionScript`))