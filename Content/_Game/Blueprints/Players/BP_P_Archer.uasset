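; BP_P_Archer is the archer player character, a child Blueprint that supplies a ranged arrow attack.
; Its AttackCollisionCheck event waits briefly to match the attack animation, then spawns a BPA_Arrow that carries the player's damage, with the archer as owner and instigator.
; The character's orientation selects the left or right shoot point and flips the arrow for left-facing shots.
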(event `self.ReceiveBeginPlay`
  (`parent.ReceiveBeginPlay`) ; Execute logics in parent class
)

(event `self.AttackCollisionCheck`
  (bind _e_orientation (`self.E_Orientation`))
  (bind _returnvalue (`SceneComponent.K2_GetComponentLocation` (`self.RightShoot`)))
  ;[0 0 0] Range Attack Collision Check
  (`KismetSystemLibrary.Delay` 0.2) ; According to your animation
  (`|SpawnActorFromClass` "/Game/_Game/Blueprints/BPA/BPA_Arrow.BPA_Arrow_C" (`KismetMathLibrary.MakeTransform` (select `/Game/_Game/Data/Enumerations/E_Orientation` _e_orientation :`NewEnumerator0` _returnvalue :`NewEnumerator1` _returnvalue :`NewEnumerator2` (`SceneComponent.K2_GetComponentLocation` (`self.LeftShoot`))) (select `/Game/_Game/Data/Enumerations/E_Orientation` _e_orientation :`NewEnumerator2` (struct :`Yaw` 180.0) :!type "Rotator Structure")) "AdjustIfPossibleButAlwaysSpawn" "MultiplyWithRoot" self self (`self.PlayerDamage`) self))

(fn `UserConstructionScript`
  (`parent.UserConstructionScript`))