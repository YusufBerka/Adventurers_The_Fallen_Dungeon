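; BP_P_Knight is the Knight player character, adding a melee attack hit check to its parent player class.
; AttackCollisionCheck runs a sphere overlap for pawns, offset left or right by the character's orientation and ignoring itself.
; Each overlapped actor tagged "enemy" receives player damage and knockback through an interface hit message.
; BeginPlay and construction defer to the parent, while debug drawing and ApplyDamage nodes are left disconnected.
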(event `self.ReceiveBeginPlay`
  (`parent.ReceiveBeginPlay`) ; Execute logics in parent class
)

(event `self.AttackCollisionCheck`
  ;[0 0 0] Melee Combat Collision Check
  (bind (_outactors _returnvalue) (`KismetSystemLibrary.SphereOverlapActors` (+ (`self.K2_GetActorLocation`) (`KismetMathLibrary.MakeVector` (select `/Game/_Game/Data/Enumerations/E_Orientation` (`self.E_Orientation`) :`NewEnumerator0` 80.0 :`NewEnumerator1` 80.0 :`NewEnumerator2` -80.0))) 80.0 (`|MakeArray` "ObjectTypeQuery3" :!type "EObjectTypeQuery Enum") null (`|MakeArray` self :!type "Actor Object Reference"))) ; Overlap enemies?
  (if _returnvalue
    (for _array_element _outactors
      (if (`self.ActorHasTag` _array_element "enemy")
        (message `/Game/_Game/Blueprints/BPI/BPI_Combat.INT_HitHandle` _array_element self (`self.PlayerDamage`) 300)))))

(fn `UserConstructionScript`
  (`parent.UserConstructionScript`))