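; Angel boss enemy for one or two players that randomly alternates between summoning minions and casting thunder.
; BOSSExtraAction saves starting HP once and starts the timer-driven attack loop, with cooldowns between skills.
; SkillA spawns wizards or ghouls at shuffled, tag-checked spawn points; SkillB repeatedly drops thunder on a random living player.
; When either skill finds no players alive, ResetBattle clears timers, restores HP and kills summoned mobs via damage interface.
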(event `self.BOSSExtraAction`
  (`/Engine/EditorBlueprintResources/StandardMacros.DoOnce` false :!label _label
    (:`Completed`
      (set `self.InitialBOSSHP` (`self.EnemyHP`))
      (`KismetSystemLibrary.K2_SetTimerDelegate` (delegate `Server_StartFighting`) 3.0) ; Activate after 5 seconds after hit
    )))

(event `ResetDoOnce`
  (goto _label :!via `Reset`))

(event `Server_StartFighting`
  (bind _returnvalue (`GameplayStatics.GetPlayerCharacter` 1))
  (bind _returnvalue_2 (`GameplayStatics.GetPlayerCharacter` 0))
  (if (`KismetSystemLibrary.IsValid` _returnvalue)
    (set `self.PlayerRefs` (`|MakeArray` _returnvalue _returnvalue_2))
    (else
      (set `self.PlayerRefs` (`|MakeArray` _returnvalue_2))))
  (set `self.isAttacking` true)
  (bind _output_get (set `self.MobIndex` (`KismetMathLibrary.RandomIntegerInRange` 0 1))) ; Store random result first
  (switch `int` _output_get
    (:`0`
      (`self.SkillA`))
    (:`1`
      (`self.SkillB`))))

(fn `CastingThunder`
  (locals (L_AlivePlayers :type "Array of Character Object Reference"))
  (bind _l_aliveplayers (`local.L_AlivePlayers`))
  (bind (_alive _liveplayers) (`self.IsAnyPlayerAlive?`))
  (if _alive
    (set `local.L_AlivePlayers` _liveplayers)
    (`KismetArrayLibrary.Array_Shuffle` _l_aliveplayers) ; Random
    (if (<= (`self.EnemyHP`) 0.0)
      (`KismetSystemLibrary.K2_ClearTimer` null "CastingThunder") ; Stop calling cycle
      (else
        (`|SpawnActorFromClass` "/Game/_Game/Blueprints/BPA/BPA_Thunder.BPA_Thunder_C" (`KismetMathLibrary.MakeTransform` (`self.K2_GetActorLocation` (`|GetArrayItem` _l_aliveplayers)) (struct) (2.0 2.0 2.0)) "AdjustIfPossibleButAlwaysSpawn" "MultiplyWithRoot" self self self)))
    (else
      (`self.ResetBattle`))))

(fn `IsAnyPlayerAlive?`
  (returns (Alive :type Boolean) (LivePlayers :type "Array of Character Object Reference"))
  (locals (L_AlivePlayers :type "Array of Character Object Reference"))
  (for _array_element (`self.PlayerRefs`)
    (bind _alive_ (message `/Game/_Game/Blueprints/BPI/BPI_Combat.INT_CheckAlive` _array_element))
    (if _alive_
      (`KismetArrayLibrary.Array_AddUnique` (`local.L_AlivePlayers`) _array_element)))
  (return (!= (`KismetArrayLibrary.Array_Length` (`local.L_AlivePlayers`)) 0) (`local.L_AlivePlayers`)))

(fn `ResetAttack`
  (set `self.isAttacking` false)
  (`KismetSystemLibrary.K2_ClearTimer` null "CastingThunder") ; Stop thunder if skill B activated
  (bind _returnvalue (`KismetSystemLibrary.K2_SetTimerDelegate` (`|CreateDelegate` :!event `Server_StartFighting`) (`KismetMathLibrary.RandomFloatInRange` 5.0 7.0))) ; Next attack
  (set `self.TimerHandle_NextAttack` _returnvalue))

(fn `ResetBattle`
  (`KismetSystemLibrary.K2_ClearTimer` null "CastingThunder") ; Stop calling cycle
  (`self.ResetAttack`)
  (`KismetSystemLibrary.K2_ClearAndInvalidateTimerHandle` (`self.TimerHandle_NextAttack`)) ; Stop next attack
  (`self.ResetDoOnce`)
  (set `self.EnemyHP` (`self.InitialBOSSHP`))
  (if (!= (`KismetArrayLibrary.Array_Length` (`self.SpawnedMobs`)) 0)
    ;[0 0 0] Destroy all spawned actors
    (for _array_element (`self.SpawnedMobs`)
      (message `/Game/_Game/Blueprints/BPI/BPI_Combat.INT_HitHandle` _array_element self 9999999.0 0))
    (`KismetArrayLibrary.Array_Clear` (`self.SpawnedMobs`))))

(fn `SkillA`
  (locals (L_SpawnLocation :type "/Game/_Game/Blueprints/BPA/BPA_SpawnMobPoints Object Reference"))
  (bind _allmobpoints (`self.AllMobPoints`))
  (bind _output (`|GetArrayItem` _allmobpoints))
  (if (not (<= (`self.EnemyHP`) 0.0))
    (bind _alive (`self.IsAnyPlayerAlive?`))
    (if _alive
      (bind _outactors (`GameplayStatics.GetAllActorsOfClass` "/Game/_Game/Blueprints/BPA/BPA_SpawnMobPoints.BPA_SpawnMobPoints_C")) ; Spawn Points
      (set `self.AllMobPoints` _outactors)
      ;[0 0 0] Spawn 3 mobs randomly among all spawn points
      (for _ (range 3)
        (`KismetArrayLibrary.Array_Shuffle` _allmobpoints) ; Randomize members in this array
        (set `local.L_SpawnLocation` _output)
        (if (`self.ActorHasTag` _output "w_p")
          (set `self.MobIndex` 0) ; wizard index
          (else
            (set `self.MobIndex` (`KismetMathLibrary.RandomIntegerInRange` 1 2))))
        (bind _returnvalue (`|SpawnActorFromClass` (select `int` (`self.MobIndex`) :`0` "/Game/_Game/Blueprints/Monsters/BP_M_Wizard.BP_M_Wizard_C" :`1` "/Game/_Game/Blueprints/Monsters/BP_M_Ghoul_Patrolling.BP_M_Ghoul_Patrolling_C" :`2` "/Game/_Game/Blueprints/Monsters/BP_M_Ghoul_Wandering.BP_M_Ghoul_Wandering_C" :!type "Actor Class Reference") (`KismetMathLibrary.MakeTransform` (`self.K2_GetActorLocation` (`local.L_SpawnLocation`)) (select `int` (`self.MobIndex`) :`0` (`self.K2_GetActorRotation` (`local.L_SpawnLocation`)) :`1` (struct) :`2` (struct))) "AdjustIfPossibleButAlwaysSpawn" "MultiplyWithRoot" null null))
        (`KismetArrayLibrary.Array_AddUnique` (`self.SpawnedMobs`) _returnvalue))
      (`KismetSystemLibrary.K2_SetTimer` null "ResetAttack" 10.0) ; Cooling down
      (else
        (`self.ResetBattle`)))))

(fn `SkillB`
  (`KismetSystemLibrary.K2_SetTimer` null "CastingThunder" 3.0 true)
  (`self.CastingThunder`) ; Instantly casting at the beginning
  (`KismetSystemLibrary.K2_SetTimer` null "ResetAttack" 10.0))

(fn `UserConstructionScript`
  (`parent.UserConstructionScript`))