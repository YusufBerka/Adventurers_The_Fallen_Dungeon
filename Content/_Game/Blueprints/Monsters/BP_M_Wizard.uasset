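; Wizard monster that periodically casts fireballs in a networked game.
; A looping three-second timer from BeginPlay calls a server event, which multicasts the firing animation override on the sprite's AnimInstance.
; SpawnFireBallOnServer, not called within this Blueprint, spawns BPA_FireBall only with authority, relying on replication to show it on clients.
; The fireball faces the sprite's yaw plus 180 degrees and carries the wizard's damage and instigator.
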(event `self.ReceiveBeginPlay`
  (`parent.ReceiveBeginPlay`)
  (`KismetSystemLibrary.K2_SetTimerDelegate` (delegate `Server_StartCasting`) 3.0 true))

(event `Server_StartCasting`
  ;[0 0 0] Broadcasting casting fireball animations to all clients
  (`self.Multicast_StartCasting`))

(event `Multicast_StartCasting`
  ;[0 0 0] Broadcasting casting fireball animations to all clients
  (`PaperZDAnimInstance.K2_PlayAnimationOverride` (`PaperZDAnimationComponent.AnimInstance` (`self.AnimationComponent`)) "/Game/_Game/Assets/Env_Monsters/wizard/AnimSequences/M_W_Fire.M_W_Fire" "DefaultSlot" 1.0 0.0))

(fn `SpawnFireBallOnServer`
  (bind (_returnvalue_roll _returnvalue_pitch _returnvalue_yaw) (`KismetMathLibrary.BreakRotator` (`SceneComponent.K2_GetComponentRotation` (`self.Sprite`))))
  (`/Engine/EditorBlueprintResources/ActorMacros.Switch Has Authority`
    (:`Authority`
      (`|SpawnActorFromClass` "/Game/_Game/Blueprints/BPA/BPA_FireBall.BPA_FireBall_C" (`KismetMathLibrary.MakeTransform` (`self.K2_GetActorLocation`) (`KismetMathLibrary.MakeRotator` 0.0 0.0 (+ _returnvalue_yaw 180.0))) "AdjustIfPossibleButAlwaysSpawn" "MultiplyWithRoot" self (`self.EnemyDamage`) self self) ; Only runs it on server, it will replicate itself on clients automatically
    )))

(fn `UserConstructionScript`
  (`parent.UserConstructionScript`))