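; Base multiplayer Paper2D enemy that takes hits from players and deals contact damage.
; Hits run an overridable boss hook, show damage text, flash the sprite red, apply optional delayed knockback away from the causer, and destroy it with VFX at zero HP.
; Server-side AttackArea overlaps damage players immediately and every second through a looping timer.
; A replicated moving flag switches idle and move flipbooks.
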(event `/Game/_Game/Blueprints/BPI/BPI_Combat.INT_HitHandle`
  (params (Causer :type "Actor Object Reference") (Damage :type "Float (double-precision)") (KnockbackForce :type Integer))
  ;[0 0 0] Handle Hit
  (`/Engine/EditorBlueprintResources/StandardMacros.IsValid` Causer
    (:`Is Valid`
      (set `self.DamageCauser` Causer)
      (set `self.ReceivedDamage` Damage)
      (set `self.Received Force` KnockbackForce)
      (`self.BOSSExtraAction`) ; Before costing hp
      (`self.Server_SpawnDmgTextActor` self (`self.ReceivedDamage`)) ; Floating damage text
      (`self.HandleHitReaction` (`self.IgnoreKnockback?`))
      (`self.HandleDeath`))))

(event `Multicast_ChangeSpriteColor`
  (params (NewColor :type "LinearColor Structure"))
  ;[0 0 0] Handle Hit
  (`PaperFlipbookComponent.SetSpriteColor` (`self.Sprite`) NewColor))

(event `BOSSExtraAction`
  ;[0 0 0] Handle Hit
  ;;[1 0 0] Overriden
)

(event `self.AttackArea.OnComponentBeginOverlap`
  (params (OverlappedComponent :type "PrimitiveComponent Object Reference") (OtherActor :type "Actor Object Reference") (OtherComp :type "PrimitiveComponent Object Reference") (OtherBodyIndex :type Integer) (bFromSweep :type Boolean) (SweepResult :type "HitResult Structure (by ref)"))
  ;[0 0 0] Cause damage
  (`/Engine/EditorBlueprintResources/ActorMacros.Switch Has Authority` ; Only server has authority to cause damage
    (:`Authority`
      (if (`self.ActorHasTag` OtherActor "player")
        (bind _returnvalue (`KismetSystemLibrary.K2_SetTimerDelegate` (delegate `ApplyDmg`) 1.0 true)) ; Keep applying damage if player character is overlapping with mob every 1 second
        (set `self.TimerHandle_CauseDamage` _returnvalue)
        (for _array_element (`PrimitiveComponent.GetOverlappingActors` (`self.AttackArea`) null) :!label _label
          (if (`self.ActorHasTag` _array_element "player")
            (message `/Game/_Game/Blueprints/BPI/BPI_Combat.INT_HitHandle` _array_element self (`self.EnemyDamage`) 0)))))))

(event `ApplyDmg`
  ;[0 0 0] Cause damage
  (goto _label))

(event `self.AttackArea.OnComponentEndOverlap`
  (params (OverlappedComponent :type "PrimitiveComponent Object Reference") (OtherActor :type "Actor Object Reference") (OtherComp :type "PrimitiveComponent Object Reference") (OtherBodyIndex :type Integer))
  ;[0 0 0] Cause damage
  (`/Engine/EditorBlueprintResources/ActorMacros.Switch Has Authority`
    (:`Authority`
      (if (and (== (`KismetArrayLibrary.Array_Length` (`PrimitiveComponent.GetOverlappingActors` (`self.AttackArea`) null)) 0) (`KismetSystemLibrary.K2_IsValidTimerHandle` (`self.TimerHandle_CauseDamage`)))
        ;;[0 0 0] Clear timer to save performance
        (`KismetSystemLibrary.K2_ClearAndInvalidateTimerHandle` (`self.TimerHandle_CauseDamage`))
        (set `self.TimerHandle_CauseDamage` (struct)) ; Optional, set this variable to NULL
      ))))

(event `Server_isMoving`
  (params (isMoving :type Boolean))
  ;[0 0 0] Moving Animation Switch
  (set `self.isMoving` isMoving))

(fn `HandleDeath`
  (if (<= (`self.EnemyHP`) 0.0)
    (`self.Server_BroadcastSound` (`self.KillSFX`) (`self.K2_GetActorLocation`))
    (`|SpawnActorFromClass` "/Game/_Game/Blueprints/BPA/BPA_VFX_MobDeath.BPA_VFX_MobDeath_C" (`KismetMathLibrary.MakeTransform` (+ (`self.K2_GetActorLocation`) (`self.MobDeathOffset`)) (struct) (`self.MobDeathScale`)) "Undefined" "MultiplyWithRoot" null null)
    (`self.K2_DestroyActor`)))

(fn `HandleHitReaction`
  (params (`DisableKB?` :type Boolean))
  (set `self.EnemyHP` (- (`self.EnemyHP`) (`self.ReceivedDamage`)))
  (set `self.isHit` true)
  (`self.Multicast_ChangeSpriteColor` (struct :`R` 1.0 :`A` 1.0))
  (`KismetSystemLibrary.K2_SetTimer` null "ResetHitColor" 0.3)
  (`KismetSystemLibrary.K2_SetTimer` null "ResetHit" 2.0)
  (`self.Server_BroadcastSound` (`self.HurtSFX`) (`self.K2_GetActorLocation`))
  (if (not (`local.DisableKB?`))
    (`KismetSystemLibrary.K2_SetTimer` null "TriggerKnockingBack" 0.1) ; Small delay is necessary for multiplayer game
  ))

(fn `INT_CheckAlive`
  (returns (`Alive?` :type Boolean))
  (return false))

(fn `OnRep_isMoving`
  (bind _idleanim (`self.IdleAnim`))
  (`/Engine/EditorBlueprintResources/StandardMacros.IsValid` _idleanim
    (:`Is Valid`
      (`PaperFlipbookComponent.SetFlipbook` (`self.Sprite`) (select `bool` (`self.isMoving`) :`false` _idleanim :`true` (`self.MoveAnim`))))))

(fn `ResetHit`
  (set `self.isHit` false))

(fn `ResetHitColor`
  (`self.Multicast_ChangeSpriteColor` (struct :`R` 1.0 :`G` 1.0 :`B` 1.0 :`A` 1.0)))

(fn `TriggerKnockingBack`
  (bind _returnvalue_x (`KismetMathLibrary.BreakVector` (`self.K2_GetActorLocation`)))
  (bind _returnvalue (`KismetMathLibrary.Conv_IntToDouble` (`self.Received Force`)))
  (`MovementComponent.StopMovementImmediately` (`self.CharacterMovement`))
  (bind _damagecauser (`self.DamageCauser`)
    (:`then`
      (bind _returnvalue_x_2 (`KismetMathLibrary.BreakVector` (`self.K2_GetActorLocation` _damagecauser)))
      (`self.LaunchCharacter` (`KismetMathLibrary.MakeVector` (select `bool` (<= _returnvalue_x_2 _returnvalue_x) :`false` (* _returnvalue -1.0) :`true` _returnvalue) 0.0 150.0) true true) ; Up 150
    )
    (:`else`)))

(fn `UserConstructionScript`
  (`parent.UserConstructionScript`))