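; Patrolling ghoul monster that walks back and forth along the X axis and chases whoever damages it.
; Tick feeds movement input at a randomized speed, while wall and floor detector overlaps flip speed and facing at walls and ledges.
; When IsHit is set, Tick switches off and AIMoveTo pursues DamageCauser, repeating after a short pause on success and re-enabling Tick on failure.
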(event `self.ReceiveBeginPlay`
  (`parent.ReceiveBeginPlay`)
  (set `self.Speed` (`KismetMathLibrary.RandomFloatInRange` 1.0 1.3)))

(event `self.ReceiveTick`
  (params (DeltaSeconds :type "Float (single-precision)"))
  ;[0 0 0] Patrol / Chase
  (`parent.ReceiveTick` DeltaSeconds)
  (`self.AddMovementInput` (0.5 0.0 0.0) (`self.Speed`))
  (if (`self.isHit`)
    (`self.SetActorTickEnabled` false)
    (`|AIMoveTo` self (0.0 0.0 0.0) (`self.DamageCauser`) :!label _label
      (:`then`
        (`self.Server_isMoving` true))
      (:`OnSuccess`
        (`self.Server_isMoving` false) ; Keep overlapping with player character
        (`KismetSystemLibrary.Delay` 2.0)
        (goto _label))
      (:`OnFail`
        ;;[0 0 0] Back to patrol
        (`self.Server_isMoving` true)
        (`self.SetActorTickEnabled` true)))))

(event `self.WallDetector.OnComponentBeginOverlap`
  (params (OverlappedComponent :type "PrimitiveComponent Object Reference") (OtherActor :type "Actor Object Reference") (OtherComp :type "PrimitiveComponent Object Reference") (OtherBodyIndex :type Integer) (bFromSweep :type Boolean) (SweepResult :type "HitResult Structure (by ref)"))
  ;[0 0 0] Check wall and cliff
  (`/Engine/EditorBlueprintResources/StandardMacros.IsValid` OtherActor
    (:`Is Valid`
      (`self.K2_SetActorRotation` (`KismetMathLibrary.MakeRotator` 0.0 0.0 (select `bool` (> (`self.Speed`) 0.0) :`true` 180.0 :!type "Float (single-precision)")) :!label _label_2)
      (set `self.Speed` (* (`self.Speed`) -1.0)))))

(event `self.FloorDetector.OnComponentEndOverlap`
  (params (OverlappedComponent :type "PrimitiveComponent Object Reference") (OtherActor :type "Actor Object Reference") (OtherComp :type "PrimitiveComponent Object Reference") (OtherBodyIndex :type Integer))
  ;[0 0 0] Check wall and cliff
  (`/Engine/EditorBlueprintResources/StandardMacros.IsValid` OtherActor
    (:`Is Valid`
      (goto _label_2))))

(fn `UserConstructionScript`
  (`parent.UserConstructionScript`))