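; BPA_FireBall is a fireball hazard actor that damages players who touch it.
; Its sphere overlap is handled only on the server and acts only on BP_PlayerBase actors that are not dead, rolling or invincible.
; A valid hit sends damage and causer through the INTHitHandleMessage interface call with no knockback, spawns the BPA_VFX_FireBallExplosion actor, then destroys the fireball.
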(event `self.Sphere.OnComponentBeginOverlap`
  (params (OverlappedComponent :type "PrimitiveComponent Object Reference") (OtherActor :type "Actor Object Reference") (OtherComp :type "PrimitiveComponent Object Reference") (OtherBodyIndex :type Integer) (bFromSweep :type Boolean) (SweepResult :type "HitResult Structure (by ref)"))
  (`/Engine/EditorBlueprintResources/ActorMacros.Switch Has Authority` ; Only runs on server side
    (:`Authority`
      (bind _asbp_player_base (cast `/Game/_Game/Blueprints/Players/BP_PlayerBase` OtherActor))
      (if (and (not (`/Game/_Game/Blueprints/Players/BP_PlayerBase.isDead` _asbp_player_base)) (not (`/Game/_Game/Blueprints/Players/BP_PlayerBase.isRolling` _asbp_player_base)) (not (`/Game/_Game/Blueprints/Players/BP_PlayerBase.isInvincible` _asbp_player_base)))
        (message `/Game/_Game/Blueprints/BPI/BPI_Combat.INT_HitHandle` OtherActor (`self.Causer`) (`self.Damage`) 0)
        (`|SpawnActorFromClass` "/Game/_Game/Blueprints/BPA/BPA_VFX_FireBallExplosion.BPA_VFX_FireBallExplosion_C" (`KismetMathLibrary.MakeTransform` (`self.K2_GetActorLocation`)) "Undefined" "MultiplyWithRoot" null null)
        (`self.K2_DestroyActor`)))))

(fn `UserConstructionScript`)