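; Thunder strike hazard actor that damages players inside its box, using the damage value of the enemy set as its causer.
; On BeginPlay, the server keeps the box's collision off for a short delay timed to the animation, then enables it and checks overlaps once.
; Players who are not dead, rolling or invincible receive a hit interface message with no knockback.
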(event `self.ReceiveBeginPlay`
  (bind _damagecauser (`self.DamageCauser`))
  (`/Engine/EditorBlueprintResources/ActorMacros.Switch Has Authority`
    (:`Authority`
      (`PrimitiveComponent.SetCollisionEnabled` (`self.Box`) "NoCollision") ; Set disabled first
      (`KismetSystemLibrary.Delay` 1.0) ; According to your animation
      (`PrimitiveComponent.SetCollisionEnabled` (`self.Box`) "QueryOnly")
      ;[0 0 0] Cause damage
      (for _array_element (`PrimitiveComponent.GetOverlappingActors` (`self.Box`) null)
        (bind _asbp_player_base (cast `/Game/_Game/Blueprints/Players/BP_PlayerBase` _array_element))
        (if (and (not (`/Game/_Game/Blueprints/Players/BP_PlayerBase.isDead` _asbp_player_base)) (not (`/Game/_Game/Blueprints/Players/BP_PlayerBase.isRolling` _asbp_player_base)) (not (`/Game/_Game/Blueprints/Players/BP_PlayerBase.isInvincible` _asbp_player_base)))
          (message `/Game/_Game/Blueprints/BPI/BPI_Combat.INT_HitHandle` _asbp_player_base _damagecauser (`/Game/_Game/Blueprints/Monsters/BP_EnemyBase.EnemyDamage` _damagecauser) 0))))))

(fn `UserConstructionScript`)